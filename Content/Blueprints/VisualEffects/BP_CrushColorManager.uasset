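; Crush mode visual manager that blends a shadow volume and a material parameter collection scalar for the player.
; On BeginPlay it binds OnTagChanged to the player's State.CrushMode gameplay tag on the ability system component and also calls it directly.
; OnTagChanged plays a timeline that drives both values.
; Its branch condition is constant true, so the timeline always restarts and the reverse path never runs.
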(event `self.ReceiveBeginPlay`
  (bind _askd_my_player (cast `kdMyPlayer` (`GameplayStatics.GetPlayerCharacter` 0)))
  (`AbilitySystemBlueprintLibrary.BindEventWrapperToGameplayTagChanged` (`AbilitySystemBlueprintLibrary.GetAbilitySystemComponent` _askd_my_player) (struct :`TagName` "State.CrushMode") (delegate `OnTagChanged`))
  (`self.OnTagChanged` (stale `OnTagChanged` Tag) (stale `OnTagChanged` TagCount)))

(event `OnTagChanged`
  (params (Tag :type "GameplayTag Structure (by ref)") (TagCount :type Integer))
  (if true
    (bind (_direction _newtrack_0) (`Timeline|Timeline_CrushBlend` :!via `PlayFromStart` :!label _label)
      (:`Update`
        (set `PostProcessVolume.BlendWeight` _newtrack_0 (`self.ShadowVolume`))
        (`KismetMaterialLibrary.SetScalarParameterValue` (`self.MPC`) (`self.Parameter Name`) _newtrack_0)))
    (else
      (goto _label :!via `Reverse`))))

(fn `UserConstructionScript`)